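; BP_InventoryTest is a functional test that checks item transfers between a Character's toolbar and inventory.
; On start it moves every toolbar item to the inventory, expecting an empty toolbar and five inventory items.
; It then adds the first inventory item to the toolbar five times, expecting the reverse counts.
; The test finishes as succeeded, or as failed with a message naming the transfer direction that broke.
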(event `self.ReceiveStartTest`
  (bind _character (`self.Character`))
  (bind _character_2 (`self.Character`))
  (bind _toolbar (`CubicalRanchCharacter.ToolBar` _character_2))
  (bind _items (`InventoryComponent.Items` (`CubicalRanchCharacter.Inventory` _character)))
  (bind _returnvalue (`ToolBarComponent.GetItems` _toolbar))
  (for _array_element _returnvalue
    (`CubicalRanchCharacter.AddItemToInventory` _character_2 _array_element))
  (bind _returnvalue_2 (`ToolBarComponent.GetItems` _toolbar))
  (if (and (== (`KismetArrayLibrary.Array_Length` _returnvalue_2) 0) (== (`KismetArrayLibrary.Array_Length` (`InventoryComponent.Items` (`CubicalRanchCharacter.Inventory` _character_2))) 5))
    (for _ (range 5)
      (`CubicalRanchCharacter.AddItemToToolBar` _character (`|GetArrayItem` _items)))
    (bind _returnvalue_3 (`ToolBarComponent.GetItems` (`CubicalRanchCharacter.ToolBar` _character)))
    (if (and (== (`KismetArrayLibrary.Array_Length` _items) 0) (== (`KismetArrayLibrary.Array_Length` _returnvalue_3) 5))
      (`self.FinishTest` "Succeeded" "Test completed succesfully")
      (else
        (`self.FinishTest` "Failed" "Items weren't added to de toolbar correctly")))
    (else
      (`self.FinishTest` "Failed" "Items weren't added to de inventory correctly"))))

(event `self.ReceiveTick`
  (params (DeltaSeconds :type "Float (single-precision)")))

(fn `UserConstructionScript`)