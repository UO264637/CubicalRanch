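; BP_AnimalTest is a functional test of the cow's feed-and-sleep day progression.
; StartTest alternates fed and unfed nights through Cow and Bed references, mostly waiting on fixed delays before checking DayCount.
; It expects the count to rise only after feeding, and to stop once the cow is Ready at two days.
; Nested checks end the test with success or a step-specific failure message.
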(event `self.ReceiveStartTest`
  (if (== (`/Game/Animals/BP_BaseAnimal.DayCount` (`self.Cow`)) 0)
    (`/Game/House/BP_Bed.Sleep` (`self.Bed`))
    (if (== (`/Game/Animals/BP_BaseAnimal.DayCount` (`self.Cow`)) 0)
      (`/Game/Animals/BP_BaseAnimal.Feed` (`self.Cow`))
      (`/Game/House/BP_Bed.Sleep` (`self.Bed`))
      (`KismetSystemLibrary.Delay` 3.5)
      (if (== (`/Game/Animals/BP_BaseAnimal.DayCount` (`self.Cow`)) 1)
        (`/Game/House/BP_Bed.Sleep` (`self.Bed`))
        (`KismetSystemLibrary.Delay` 3.5)
        (if (== (`/Game/Animals/BP_BaseAnimal.DayCount` (`self.Cow`)) 1)
          (`/Game/Animals/BP_BaseAnimal.Feed` (`self.Cow`))
          (`/Game/House/BP_Bed.Sleep` (`self.Bed`))
          (`KismetSystemLibrary.Delay` 3.5)
          (if (== (`/Game/Animals/BP_BaseAnimal.DayCount` (`self.Cow`)) 2)
            (`/Game/House/BP_Bed.Sleep` (`self.Bed`))
            (`KismetSystemLibrary.Delay` 3.5)
            (if (== (`/Game/Animals/BP_BaseAnimal.DayCount` (`self.Cow`)) 2)
              (if (`/Game/Animals/BP_BaseAnimal.Ready` (`self.Cow`))
                (`/Game/Animals/BP_BaseAnimal.Feed` (`self.Cow`))
                (`/Game/House/BP_Bed.Sleep` (`self.Bed`))
                (`KismetSystemLibrary.Delay` 3.5)
                (if (== (`/Game/Animals/BP_BaseAnimal.DayCount` (`self.Cow`)) 2)
                  (`/Game/House/BP_Bed.Sleep` (`self.Bed`))
                  (`KismetSystemLibrary.Delay` 3.5)
                  (if (== (`/Game/Animals/BP_BaseAnimal.DayCount` (`self.Cow`)) 2)
                    (`self.FinishTest` "Succeeded")
                    (else
                      (`self.FinishTest` "Failed" "Day count should be 2 (already redy no feed)")))
                  (else
                    (`self.FinishTest` "Failed" "Day count should be 2 (already ready)")))
                (else
                  (`self.FinishTest` "Failed" "Cow should be ready")))
              (else
                (`self.FinishTest` "Failed" "Day count should be 2 (no feed)")))
            (else
              (`self.FinishTest` "Failed" "Day count should be 2")))
          (else
            (`self.FinishTest` "Failed" "Day count should be 1 (no feed)")))
        (else
          (`self.FinishTest` "Failed" "Day count should be 1")))
      (else
        (`self.FinishTest` "Failed" "Day count should be 0")))
    (else
      (`self.FinishTest` "Failed" "Initial day count should be 0"))))

(fn `UserConstructionScript`)