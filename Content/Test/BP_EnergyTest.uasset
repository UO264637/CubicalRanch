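; Functional test that checks the character's energy system against sleeping, spending and exhaustion.
; StartTest sleeps in the bed, waits, and confirms energy is at max, then spends some and sleeps again to check the refill.
; It then drains energy to zero in fixed steps and, after a delay without calling Sleep, expects day 3 with half energy.
; Each failed check reports through FinishTest with a message.
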(event `self.ReceivePrepareTest`)

(event `self.ReceiveStartTest`
  (bind _character (`self.Character`))
  (bind _character_2 (`self.Character`))
  (bind _character_3 (`self.Character`))
  (bind _character_4 (`self.Character`))
  (bind _character_5 (`self.Character`))
  (`/Game/House/BP_Bed.Sleep` (`self.Bed`))
  (`KismetSystemLibrary.Delay` 3.5)
  (if (== (`CubicalRanchCharacter.MAX_ENERGY` _character) (`CubicalRanchCharacter.Energy` _character))
    (`/Game/BP_CubicalRanchCharacter.SpendEnergy` (`self.Character`) 5)
    (if (not (== (- (`CubicalRanchCharacter.MAX_ENERGY` _character_3) 5) (`CubicalRanchCharacter.Energy` _character_3)))
      (`self.FinishTest` "Failed" "Energy should be at 195"))
    (`/Game/House/BP_Bed.Sleep` (`self.Bed`))
    (`KismetSystemLibrary.Delay` 3.5)
    (if (== (`CubicalRanchCharacter.MAX_ENERGY` _character_5) (`CubicalRanchCharacter.Energy` _character_5))
      (for _ (range (+ (- (/ (`CubicalRanchCharacter.MAX_ENERGY` (`self.Character`)) 5) 2) 1))
        (`/Game/BP_CubicalRanchCharacter.SpendEnergy` _character_4 5))
      (if (== (`CubicalRanchCharacter.Energy` _character_4) 5)
        (`/Game/BP_CubicalRanchCharacter.SpendEnergy` (`self.Character`) 5)
        (if (== (`CubicalRanchCharacter.Energy` (`self.Character`)) 0)
          (`KismetSystemLibrary.Delay` 4.0)
          (if (and (== (`/Game/BP_CubicalRanchCharacter.Day` _character_2) 3) (== (`CubicalRanchCharacter.Energy` _character_2) (/ (`CubicalRanchCharacter.MAX_ENERGY` _character_2) 2)))
            (`self.FinishTest` "Succeeded")
            (else
              (`self.FinishTest` "Failed" "Energy should be at half and day should hav passed")))
          (else
            (`self.FinishTest` "Failed" "Energy should be 0")))
        (else
          (`self.FinishTest` "Failed" "Energy should be 5")))
      (else
        (`self.FinishTest` "Failed" "Energy should be at max (after spent)")))
    (else
      (`self.FinishTest` "Failed" "Energy should be at max"))))

(fn `UserConstructionScript`)