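; Functional test that checks wheat crop growth through stages 0 to 4 on a soil actor.
; It plants a new wheat seed, then alternates dry and watered nights by sleeping in a bed, mostly with delays between steps, expecting growth only after watering.
; At the cap, it checks that the seed's stage object stays "wheat4".
; The first mismatch fails the test, usually naming the expected stage.
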(event `self.ReceiveStartTest`
  (bind _soil (`self.Soil`))
  (bind _returnvalue (`|GenericCreateObject` "/Game/InventorySystem/BP_WheatSeed.BP_WheatSeed_C" self))
  (bind _output_get (set `self.Wheat Seed` _returnvalue))
  (`/Game/Blocks/BP_Block.PlantSeed` _soil _output_get)
  (if (== (`/Game/Blocks/BP_Soil.Stage` _soil) 0)
    (`/Game/House/BP_Bed.Sleep` (`self.Bed`))
    (if (== (`/Game/Blocks/BP_Soil.Stage` (`self.Soil`)) 0)
      (`/Game/Blocks/BP_Block.Water` (`self.Soil`))
      (`/Game/House/BP_Bed.Sleep` (`self.Bed`))
      (`KismetSystemLibrary.Delay` 3.5)
      (if (== (`/Game/Blocks/BP_Soil.Stage` (`self.Soil`)) 1)
        (`/Game/House/BP_Bed.Sleep` (`self.Bed`))
        (`KismetSystemLibrary.Delay` 3.5)
        (if (== (`/Game/Blocks/BP_Soil.Stage` (`self.Soil`)) 1)
          (`/Game/Blocks/BP_Block.Water` (`self.Soil`))
          (`/Game/House/BP_Bed.Sleep` (`self.Bed`))
          (`KismetSystemLibrary.Delay` 3.5)
          (if (== (`/Game/Blocks/BP_Soil.Stage` (`self.Soil`)) 2)
            (`/Game/House/BP_Bed.Sleep` (`self.Bed`))
            (`KismetSystemLibrary.Delay` 3.5)
            (if (== (`/Game/Blocks/BP_Soil.Stage` (`self.Soil`)) 2)
              (`/Game/Blocks/BP_Block.Water` (`self.Soil`))
              (`/Game/House/BP_Bed.Sleep` (`self.Bed`))
              (`KismetSystemLibrary.Delay` 3.5)
              (if (== (`/Game/Blocks/BP_Soil.Stage` (`self.Soil`)) 3)
                (`/Game/House/BP_Bed.Sleep` (`self.Bed`))
                (`KismetSystemLibrary.Delay` 3.5)
                (if (== (`/Game/Blocks/BP_Soil.Stage` (`self.Soil`)) 3)
                  (`/Game/Blocks/BP_Block.Water` (`self.Soil`))
                  (`/Game/House/BP_Bed.Sleep` (`self.Bed`))
                  (`KismetSystemLibrary.Delay` 3.5)
                  (if (== (`/Game/Blocks/BP_Soil.Stage` (`self.Soil`)) 4)
                    (`/Game/House/BP_Bed.Sleep` (`self.Bed`))
                    (`KismetSystemLibrary.Delay` 3.5)
                    (if (== (`/Game/Blocks/BP_Soil.Stage` (`self.Soil`)) 4)
                      (`/Game/Blocks/BP_Block.Water` (`self.Soil`))
                      (`/Game/House/BP_Bed.Sleep` (`self.Bed`))
                      (`KismetSystemLibrary.Delay` 3.5)
                      (bind _returnvalue_2 (`SeedItem.GetStage` (`self.Wheat Seed`) (`/Game/Blocks/BP_Soil.Stage` (`self.Soil`))))
                      (if (`KismetStringLibrary.EqualEqual_StrStr` (`KismetSystemLibrary.GetObjectName` _returnvalue_2) "wheat4")
                        (`/Game/House/BP_Bed.Sleep` (`self.Bed`))
                        (`KismetSystemLibrary.Delay` 3.5)
                        (bind _returnvalue_3 (`SeedItem.GetStage` (`self.Wheat Seed`) (`/Game/Blocks/BP_Soil.Stage` (`self.Soil`))))
                        (if (`KismetStringLibrary.EqualEqual_StrStr` (`KismetSystemLibrary.GetObjectName` _returnvalue_3) "wheat4")
                          (`self.FinishTest` "Succeeded")
                          (else
                            (`self.FinishTest` "Failed" "Stage should be 4 max growing (no water)")))
                        (else
                          (`self.FinishTest` "Failed" "Stage should be 4 max growth")))
                      (else
                        (`self.FinishTest` "Failed" "Stage should be 4 (no water)")))
                    (else
                      (`self.FinishTest` "Failed" "Stage should be 4")))
                  (else
                    (`self.FinishTest` "Failed" "Stage should be 3 (no water)")))
                (else
                  (`self.FinishTest` "Failed" "Stage should be 3")))
              (else
                (`self.FinishTest` "Failed" "Stage should be 2 (no water)")))
            (else
              (`self.FinishTest` "Failed" "Stage should be 2")))
          (else
            (`self.FinishTest` "Failed" "Stage should be 1 (no water)")))
        (else
          (`self.FinishTest` "Failed" "Stage should be 1")))
      (else
        (`self.FinishTest` "Failed" "Stage should be 0")))
    (else
      (`self.FinishTest` "Failed" "Initial stage should be 0"))))

(fn `UserConstructionScript`)