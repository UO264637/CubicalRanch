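; BP_Cow is a farm animal that gives the player milk when clicked while its product is ready.
; On BeginPlay it sets a two-day production period and hands off to the parent class, as day counting is not handled here.
; Clicking the mesh constructs a BP_Milk, gives it to the FemaleCharacter player, then clears the ready flag, resets the day count and updates the text render.
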(event `self.ReceiveBeginPlay`
  (set `self.ProductionDays` 2)
  (`parent.ReceiveBeginPlay`))

(event `self.Mesh.OnClicked`
  (params (TouchedComponent :type "PrimitiveComponent Object Reference") (ButtonPressed :type "Key Structure"))
  (if (`self.Ready`)
    (bind _returnvalue (`|GenericCreateObject` "/Game/InventorySystem/BP_Milk.BP_Milk_C" "BP_Cow"))
    (bind _asfemale_character (cast `/Game/FemaleCharacter` (`GameplayStatics.GetPlayerCharacter` 0)))
    (`CubicalRanchCharacter.GiveItem` _asfemale_character _returnvalue 1)
    (set `self.Ready` false)
    (set `self.DayCount` 0)
    (`TextRenderComponent.K2_SetText` (`self.TextRender1`) (`self.Text`))))

(fn `UserConstructionScript`
  (`parent.UserConstructionScript`))