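; BP_Chicken is a farm animal that produces an egg after being fed.
; Each Grow call advances a day counter while Fed is set; on reaching ProductionDays it spawns a BP_EggActor at its own transform, then resets the counter and Fed.
; BeginPlay sets a one-day production period and prints the controller's display name as debug output.
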(event `/Game/Animals/GrowingInterface.Grow`
  (if (`self.Fed`)
    (`/Engine/EditorBlueprintResources/StandardMacros.IncrementInt` (`self.DayCount`)
      (:`  `
        (if (>= (`self.DayCount`) (`self.ProductionDays`))
          (`|SpawnActorFromClass` "/Game/Animals/BP_EggActor.BP_EggActor_C" (`self.GetTransform`) "Undefined" "OverrideRootScale" null null)
          (set `self.DayCount` 0)
          (set `self.Fed` false))))))

(event `self.ReceiveBeginPlay`
  (set `self.ProductionDays` 1)
  (`KismetSystemLibrary.PrintString` (`KismetSystemLibrary.GetDisplayName` (`self.GetController`))))

(fn `UserConstructionScript`
  (`parent.UserConstructionScript`))