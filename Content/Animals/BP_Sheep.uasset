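; BP_Sheep is a ranch animal that yields wool on a production cycle, set to seven days at BeginPlay before calling the parent.
; Clicking a ready sheep gives the player a wool item, spends energy, advances achievements and resets the cycle.
; Shearing plays a sound and briefly halts the sheep and disables player input while the MilkingShearing flag is set, then restores NavWalking and input.
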(event `self.ReceiveBeginPlay`
  (set `self.ProductionDays` 7)
  (`parent.ReceiveBeginPlay`))

(event `self.Mesh.OnClicked`
  (params (TouchedComponent :type "PrimitiveComponent Object Reference") (ButtonPressed :type "Key Structure"))
  (bind _returnvalue (`GameplayStatics.GetPlayerController` 0))
  (if (`self.Ready`)
    (bind _returnvalue_2 (`|GenericCreateObject` "/Game/InventorySystem/BP_Wool.BP_Wool_C" "BP_Sheep"))
    (bind _asbp_cubical_ranch_character (cast `/Game/BP_CubicalRanchCharacter` (`GameplayStatics.GetPlayerCharacter` 0)))
    (`/Game/BP_CubicalRanchCharacter.ProgressAchievement` _asbp_cubical_ranch_character "WOOL" 1)
    (`/Game/BP_CubicalRanchCharacter.ProgressAchievement` _asbp_cubical_ranch_character "PRODUCTS" 1)
    (`/Game/BP_CubicalRanchCharacter.SpendEnergy` _asbp_cubical_ranch_character 5)
    (`CubicalRanchCharacter.GiveItem` _asbp_cubical_ranch_character _returnvalue_2 1)
    (set `self.Ready` false)
    (set `self.DayCount` 0)
    (`TextRenderComponent.K2_SetText` (`self.TextRender1`) (`self.Text`))
    (`GameplayStatics.PlaySoundAtLocation` "/Game/MyAssets/Sounds/Shear.Shear" (`self.K2_GetActorLocation`) (struct) 1.0 1.0 0.0 null null null)
    (`CharacterMovementComponent.DisableMovement` (`self.CharacterMovement`))
    (`self.DisableInput` _asbp_cubical_ranch_character _returnvalue)
    (set `/Game/BP_CubicalRanchCharacter.MilkingShearing` true _asbp_cubical_ranch_character)
    (`KismetSystemLibrary.Delay` 0.8)
    (set `/Game/BP_CubicalRanchCharacter.MilkingShearing` false _asbp_cubical_ranch_character)
    (`self.EnableInput` _asbp_cubical_ranch_character _returnvalue)
    (`CharacterMovementComponent.SetMovementMode` (`self.CharacterMovement`) "MOVE_NavWalking" 0)))

(fn `UserConstructionScript`
  (`parent.UserConstructionScript`))