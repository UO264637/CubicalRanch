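; Base farm animal for the ranch game that can be fed and becomes ready to produce after enough fed days.
; Feed succeeds once until Grow resets it, costing player energy, advancing the FEED achievement and playing heart particles and sound.
; Grow counts only fed days toward ProductionDays, then sets Ready and updates its text label.
; Tick calls Jump while moving for a hopping gait, and cursor hover toggles a custom-depth stencil outline.
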(event `/Game/Animals/GrowingInterface.Grow`
  (if (`self.Fed`)
    (set `self.Fed` false)
    (if (not (`self.Ready`))
      (`/Engine/EditorBlueprintResources/StandardMacros.IncrementInt` (`self.DayCount`)
        (:`  `
          (if (>= (`self.DayCount`) (`self.ProductionDays`))
            (set `self.Ready` true)
            (`TextRenderComponent.K2_SetText` (`self.TextRender1`) (`self.ReadyText`))))))))

(event `self.ReceiveBeginPlay`)

(event `self.ReceiveTick`
  (params (DeltaSeconds :type "Float (single-precision)"))
  (bind (_returnvalue_x _returnvalue_y) (`KismetMathLibrary.BreakVector` (`self.GetVelocity`)))
  (if (or (> (`KismetMathLibrary.Abs` _returnvalue_x) 30.0) (> (`KismetMathLibrary.Abs` _returnvalue_y) 30.0))
    (`self.Jump`)))

(event `self.Mesh.OnBeginCursorOver`
  (params (TouchedComponent :type "PrimitiveComponent Object Reference"))
  (bind _mesh (`self.Mesh`))
  ;[1 1 1] Outline
  (`PrimitiveComponent.SetRenderCustomDepth` _mesh true)
  (`PrimitiveComponent.SetCustomDepthStencilValue` _mesh 2))

(event `self.Mesh.OnEndCursorOver`
  (params (TouchedComponent :type "PrimitiveComponent Object Reference"))
  (bind _mesh (`self.Mesh`))
  ;[1 1 1] Outline
  (`PrimitiveComponent.SetRenderCustomDepth` _mesh false)
  (`PrimitiveComponent.SetCustomDepthStencilValue` _mesh 0))

(fn `Feed`
  (returns (Success :type Boolean))
  (bind _returnvalue (`self.K2_GetActorLocation`))
  (if (`self.Fed`)
    (return false)
    (else
      (set `self.Fed` true)
      (bind _asbp_cubical_ranch_character (cast `/Game/BP_CubicalRanchCharacter` (`GameplayStatics.GetPlayerCharacter` 0)))
      (`/Game/BP_CubicalRanchCharacter.ProgressAchievement` _asbp_cubical_ranch_character "FEED" 1)
      (`/Game/BP_CubicalRanchCharacter.SpendEnergy` _asbp_cubical_ranch_character 5)
      (`GameplayStatics.SpawnEmitterAtLocation` "/Game/MyAssets/Materials/HeartParticleSystem.HeartParticleSystem" _returnvalue (struct) (1.5 1.5 1.5))
      (`GameplayStatics.PlaySoundAtLocation` "/Game/MyAssets/Sounds/Feed.Feed" _returnvalue (struct) 1.0 1.0 0.0 null null null)
      (return true))))

(fn `UserConstructionScript`)