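; BP_HouseFurniture is an interactable house furniture actor that responds to the mouse when the player character is within 350 units.
; Cursor hover toggles custom depth and stencil on the static mesh for an outline, with the same range check on both enter and exit.
; Clicking in range calls DoAction, which is empty here and appears to be a hook for child Blueprints.
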(event `self.StaticMesh.OnBeginCursorOver`
  (params (TouchedComponent :type "PrimitiveComponent Object Reference"))
  (bind _returnvalue_location (`KismetMathLibrary.BreakTransform` (`self.GetTransform`)))
  (bind _staticmesh (`self.StaticMesh`))
  (bind _returnvalue_location_2 (`KismetMathLibrary.BreakTransform` (`self.GetTransform` (`GameplayStatics.GetPlayerCharacter` 0))))
  ;[1 1 1] Outine
  (if (< (`KismetMathLibrary.VSize` (- _returnvalue_location_2 _returnvalue_location)) 350.0)
    (`PrimitiveComponent.SetRenderCustomDepth` _staticmesh true)
    (`PrimitiveComponent.SetCustomDepthStencilValue` _staticmesh 2)))

(event `self.StaticMesh.OnEndCursorOver`
  (params (TouchedComponent :type "PrimitiveComponent Object Reference"))
  (bind _returnvalue_location (`KismetMathLibrary.BreakTransform` (`self.GetTransform`)))
  (bind _staticmesh (`self.StaticMesh`))
  (bind _returnvalue_location_2 (`KismetMathLibrary.BreakTransform` (`self.GetTransform` (`GameplayStatics.GetPlayerCharacter` 0))))
  ;[1 1 1] Outine
  (if (< (`KismetMathLibrary.VSize` (- _returnvalue_location_2 _returnvalue_location)) 350.0)
    (`PrimitiveComponent.SetRenderCustomDepth` _staticmesh false)
    (`PrimitiveComponent.SetCustomDepthStencilValue` _staticmesh 0)))

(event `self.ReceiveActorOnClicked`
  (params (ButtonPressed :type "Key Structure"))
  (bind _returnvalue_location (`KismetMathLibrary.BreakTransform` (`self.GetTransform`)))
  (bind _returnvalue_location_2 (`KismetMathLibrary.BreakTransform` (`self.GetTransform` (`GameplayStatics.GetPlayerCharacter` 0))))
  (if (< (`KismetMathLibrary.VSize` (- _returnvalue_location_2 _returnvalue_location)) 350.0)
    (`self.DoAction`)))

(fn `DoAction`)

(fn `UserConstructionScript`)