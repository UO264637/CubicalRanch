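; BP_Bed is a clickable bed that lets the player sleep to recover energy and pass the day.
; Clicking its mesh disables input, teleports the pawn to the SleepPosition component and calls RecoverEnergy on the BP_CubicalRanchCharacter.
; After a short delay it teleports the pawn to the Stand component, restores input and calls the pass-day dispatcher.
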(event `self.StaticMesh.OnClicked`
  (params (TouchedComponent :type "PrimitiveComponent Object Reference") (ButtonPressed :type "Key Structure"))
  (bind _returnvalue (`GameplayStatics.GetPlayerPawn` 0))
  (bind _returnvalue_2 (`GameplayStatics.GetPlayerController` 0))
  (bind _sleepposition (`self.SleepPosition`))
  (bind _stand (`self.Stand`))
  (`self.DisableInput` _returnvalue _returnvalue_2)
  (`self.K2_TeleportTo` _returnvalue (`SceneComponent.K2_GetComponentLocation` _sleepposition) (`SceneComponent.K2_GetComponentRotation` _sleepposition))
  (bind _asbp_cubical_ranch_character (cast `/Game/BP_CubicalRanchCharacter` _returnvalue))
  (`/Game/BP_CubicalRanchCharacter.RecoverEnergy` _asbp_cubical_ranch_character)
  (`KismetSystemLibrary.Delay` 3.0)
  (`self.K2_TeleportTo` _returnvalue (`SceneComponent.K2_GetComponentLocation` _stand) (`SceneComponent.K2_GetComponentRotation` _stand))
  (`self.EnableInput` _returnvalue _returnvalue_2)
  (`self.PassDayDispatcher`))

(fn `UserConstructionScript`)