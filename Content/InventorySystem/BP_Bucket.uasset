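; BP_Bucket is an inventory tool that adds and removes water blocks in the block world.
; Left use on a BP_Grass block destroys it, has the ranch character place BP_Water at its transform, then updates the new block.
; Right use on grass deletes the block on top of it if that block is water.
; Both successful actions play a water sound and the tool animation.
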(event `self.OnLeftUse`
  (params (Character :type "CubicalRanchCharacter Object Reference") (location :type "Transform Structure") (HitActor :type "Actor Object Reference"))
  (bind _asbp_cubical_ranch_character (cast `/Game/BP_CubicalRanchCharacter` Character))
  (bind _asbp_grass (cast `/Game/Blocks/BP_Grass` HitActor))
  (bind _output_get (set `self.PreviousTransform` (`Actor.GetTransform` _asbp_grass)))
  (`Actor.K2_DestroyActor` _asbp_grass)
  (bind _placedblock (`/Game/BP_CubicalRanchCharacter.PlaceBlock` _asbp_cubical_ranch_character "/Game/Blocks/BP_Water.BP_Water_C" _output_get))
  (`/Game/Blocks/BP_Block.Update` _placedblock null)
  (`/Game/BP_CubicalRanchCharacter.PlaySound` _asbp_cubical_ranch_character "/Game/MyAssets/Sounds/Water.Water" location_Location)
  (`self.PlayToolAnimation` Character))

(event `self.OnRightUse`
  (params (Character :type "CubicalRanchCharacter Object Reference") (location :type "Transform Structure") (HitActor :type "Actor Object Reference"))
  (bind _asbp_cubical_ranch_character (cast `/Game/BP_CubicalRanchCharacter` Character))
  (bind _asbp_grass (cast `/Game/Blocks/BP_Grass` HitActor))
  (bind _actor (`/Game/Blocks/BP_Block.GetTopBlock` _asbp_grass))
  (bind _asbp_water (cast `/Game/Blocks/BP_Water` _actor))
  (`/Game/Blocks/BP_Block.Delete` _asbp_water)
  (`/Game/BP_CubicalRanchCharacter.PlaySound` _asbp_cubical_ranch_character "/Game/MyAssets/Sounds/Water.Water" location_Scale)
  (`self.PlayToolAnimation` Character))