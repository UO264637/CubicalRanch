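; BP_Shovel is an inventory tool that places and removes Grass blocks in the world.
; Left use has the FemaleCharacter place a Grass block at the given location when the hit actor is Terrain, or Grass without Water as its top block.
; Right use destroys a hit Grass actor, unless its top block is Water.
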(event `self.OnLeftUse`
  (params (Character :type "CubicalRanchCharacter Object Reference") (location :type "Transform Structure") (HitActor :type "Actor Object Reference"))
  (bind _asfemale_character (cast `/Game/FemaleCharacter` Character))
  (cast `/Game/Terrain` HitActor
    (:`then`
      _)
    (:`CastFailed`
      (bind _asgrass (cast `/Game/Blocks/Grass` HitActor))
      (bind _actor (`/Game/Blocks/Block.GetTopBlock` _asgrass))
      (cast `/Game/Blocks/Water` _actor
        (:`CastFailed`
          _))))
  (`/Game/FemaleCharacter.PlaceBlock` _asfemale_character "/Game/Blocks/Grass.Grass_C" location))

(event `self.OnRightUse`
  (params (Character :type "CubicalRanchCharacter Object Reference") (location :type "Transform Structure") (HitActor :type "Actor Object Reference"))
  (bind _asgrass (cast `/Game/Blocks/Grass` HitActor))
  (bind _actor (`/Game/Blocks/Block.GetTopBlock` _asgrass))
  (cast `/Game/Blocks/Water` _actor
    (:`CastFailed`
      (`Actor.K2_DestroyActor` HitActor))))