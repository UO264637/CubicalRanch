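; BP_Hoe is an inventory tool that converts ground blocks between grass and soil, costing the player energy.
; Left use turns a Grass actor into Soil2, and right use turns Soil2 back into Grass.
; Each use casts the user to FemaleCharacter, destroys the hit block, then has the character place the replacement at the saved transform and spend energy.
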(event `self.OnLeftUse`
  (params (Character :type "CubicalRanchCharacter Object Reference") (location :type "Transform Structure") (HitActor :type "Actor Object Reference"))
  (bind _asfemale_character (cast `/Game/FemaleCharacter` Character))
  (bind _asgrass (cast `/Game/Blocks/Grass` HitActor))
  (set `self.PreviousTransform` (`Actor.GetTransform` _asgrass))
  (`Actor.K2_DestroyActor` HitActor)
  (`/Game/FemaleCharacter.PlaceBlock` _asfemale_character "/Game/Blocks/Soil2.Soil2_C" (`self.PreviousTransform`))
  (`/Game/FemaleCharacter.SpendEnergy` _asfemale_character 5))

(event `self.OnRightUse`
  (params (Character :type "CubicalRanchCharacter Object Reference") (location :type "Transform Structure") (HitActor :type "Actor Object Reference"))
  (bind _asfemale_character (cast `/Game/FemaleCharacter` Character))
  (bind _assoil_2 (cast `/Game/Blocks/Soil2` HitActor))
  (set `self.PreviousTransform` (`Actor.GetTransform` _assoil_2))
  (`Actor.K2_DestroyActor` _assoil_2)
  (`/Game/FemaleCharacter.PlaceBlock` _asfemale_character "/Game/Blocks/Grass.Grass_C" (`self.PreviousTransform`))
  (`/Game/FemaleCharacter.SpendEnergy` _asfemale_character 5))