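; BP_ChickenPurchase is an inventory item for buying chickens, supplying chicken-specific pieces of the purchase.
; GetAnimals returns every BP_Chicken in the level, and ShowMessage tells the player character that the chicken limit is reached.
; An unconnected older graph gathers unpurchased chickens, teleports them to the farm and removes the item, but it never runs.
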(event `self.ShowMessage`
  (bind _asbp_cubical_ranch_character (cast `/Game/BP_CubicalRanchCharacter` (`GameplayStatics.GetPlayerCharacter` 0)))
  (`/Game/BP_CubicalRanchCharacter.ShowMessage` _asbp_cubical_ranch_character "Reached limit of chickens"))

(fn `GetAnimals`
  (returns (Animals :type "Array of /Game/Animals/BP_BaseAnimal Object Reference"))
  (bind _outactors (`GameplayStatics.GetAllActorsOfClass` "/Game/Animals/BP_Chicken.BP_Chicken_C"))
  (return _outactors))