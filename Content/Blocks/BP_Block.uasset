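; Base-style block actor that highlights under the cursor and can look up adjacent blocks.
; Cursor hover toggles the mesh's custom depth and stencil value, presumably for an outline effect.
; Six getters each line-trace one block length along a world axis to return the neighboring actor; the bottom trace leaves persistent debug lines.
; Update, Delete and PlantSeed are stubs, with PlantSeed always returning false.
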(event `self.StaticMesh.OnBeginCursorOver`
  (params (TouchedComponent :type "PrimitiveComponent Object Reference"))
  (bind _staticmesh (`self.StaticMesh`))
  (`PrimitiveComponent.SetRenderCustomDepth` _staticmesh true)
  (`PrimitiveComponent.SetCustomDepthStencilValue` _staticmesh 2))

(event `self.StaticMesh.OnEndCursorOver`
  (params (TouchedComponent :type "PrimitiveComponent Object Reference"))
  (bind _staticmesh (`self.StaticMesh`))
  (`PrimitiveComponent.SetRenderCustomDepth` _staticmesh false)
  (`PrimitiveComponent.SetCustomDepthStencilValue` _staticmesh 0))

(fn `Delete`)

(fn `GetBackBlock`
  (returns (Actor :type "Actor Object Reference"))
  (bind (_returnvalue_x _returnvalue_y _returnvalue_z) (`KismetMathLibrary.BreakVector` (`self.K2_GetActorLocation`)))
  (bind _outhit (`KismetSystemLibrary.LineTraceSingleForObjects` (`self.K2_GetActorLocation`) (`KismetMathLibrary.MakeVector` (+ _returnvalue_x 100.0) _returnvalue_y _returnvalue_z) (`self.NewVar_0`)))
  (return (`.HitActor` (`GameplayStatics.BreakHitResult` _outhit))))

(fn `GetBottomBlock`
  (returns (Actor :type "Actor Object Reference"))
  (bind (_returnvalue_x _returnvalue_y _returnvalue_z) (`KismetMathLibrary.BreakVector` (`self.K2_GetActorLocation`)))
  (bind _outhit (`KismetSystemLibrary.LineTraceSingleForObjects` :`Start` (`self.K2_GetActorLocation`) :`End` (`KismetMathLibrary.MakeVector` _returnvalue_x _returnvalue_y (- _returnvalue_z 100.0)) :`ObjectTypes` (`self.NewVar_0`) :`DrawDebugType` "Persistent"))
  (return (`.HitActor` (`GameplayStatics.BreakHitResult` _outhit))))

(fn `GetFrontBlock`
  (returns (Actor :type "Actor Object Reference"))
  (bind (_returnvalue_x _returnvalue_y _returnvalue_z) (`KismetMathLibrary.BreakVector` (`self.K2_GetActorLocation`)))
  (bind _outhit (`KismetSystemLibrary.LineTraceSingleForObjects` (`self.K2_GetActorLocation`) (`KismetMathLibrary.MakeVector` (- _returnvalue_x 100.0) _returnvalue_y _returnvalue_z) (`self.NewVar_0`)))
  (return (`.HitActor` (`GameplayStatics.BreakHitResult` _outhit))))

(fn `GetLeftBlock`
  (returns (Actor :type "Actor Object Reference"))
  (bind (_returnvalue_x _returnvalue_y _returnvalue_z) (`KismetMathLibrary.BreakVector` (`self.K2_GetActorLocation`)))
  (bind _outhit (`KismetSystemLibrary.LineTraceSingleForObjects` (`self.K2_GetActorLocation`) (`KismetMathLibrary.MakeVector` _returnvalue_x (- _returnvalue_y 100.0) _returnvalue_z) (`self.NewVar_0`)))
  (return (`.HitActor` (`GameplayStatics.BreakHitResult` _outhit))))

(fn `GetRightBlock`
  (returns (Actor :type "Actor Object Reference"))
  (bind (_returnvalue_x _returnvalue_y _returnvalue_z) (`KismetMathLibrary.BreakVector` (`self.K2_GetActorLocation`)))
  (bind _outhit (`KismetSystemLibrary.LineTraceSingleForObjects` (`self.K2_GetActorLocation`) (`KismetMathLibrary.MakeVector` _returnvalue_x (+ _returnvalue_y 100.0) _returnvalue_z) (`self.NewVar_0`)))
  (return (`.HitActor` (`GameplayStatics.BreakHitResult` _outhit))))

(fn `GetTopBlock`
  (returns (Actor :type "Actor Object Reference"))
  (bind (_returnvalue_x _returnvalue_y _returnvalue_z) (`KismetMathLibrary.BreakVector` (`self.K2_GetActorLocation`)))
  (bind _outhit (`KismetSystemLibrary.LineTraceSingleForObjects` (`self.K2_GetActorLocation`) (`KismetMathLibrary.MakeVector` _returnvalue_x _returnvalue_y (+ _returnvalue_z 100.0)) (`self.NewVar_0`)))
  (return (`.HitActor` (`GameplayStatics.BreakHitResult` _outhit))))

(fn `PlantSeed`
  (params (SeedItem :type "SeedItem Object Reference"))
  (returns (Succes :type Boolean))
  (return false))

(fn `Update`
  (params (Block :type "/Game/Blocks/BP_Block Object Reference")))

(fn `UserConstructionScript`)