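; Farm soil block that the player plants, waters and harvests, tracking one seed item and its growth stage.
; PlantSeed spawns a crop mesh component at runtime, and Water switches the soil to its watered mesh.
; Grow always dries the soil, advancing the crop's stage mesh and binding its click only if watered.
; Clicking a mature crop spends energy, gives the product and clears the plot; planting, watering and harvesting progress achievements.
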(event `/Game/Blocks/BlockInterface.Water`
  (if (not (`self.IsWatered`))
    (set `self.IsWatered` true)
    (`StaticMeshComponent.SetStaticMesh` (`self.StaticMesh`) "/Game/MyAssets/blocks/WateredSoil.WateredSoil")
    (bind _asbp_cubical_ranch_character (cast `/Game/BP_CubicalRanchCharacter` (`GameplayStatics.GetPlayerCharacter` 0)))
    (`/Game/BP_CubicalRanchCharacter.ProgressAchievement` _asbp_cubical_ranch_character "WATER" 1)))

(event `/Game/Animals/GrowingInterface.Grow`
  (bind _staticmesh (`self.StaticMesh`))
  (bind _crop (`self.Crop`))
  (if (and (`KismetSystemLibrary.IsValid` (`self.SeedItem`)) (`self.IsWatered`))
    (`/Engine/EditorBlueprintResources/StandardMacros.IncrementInt` (`self.Stage`)
      (:`  `
        (`StaticMeshComponent.SetStaticMesh` _staticmesh "/Game/MyAssets/blocks/soil.soil")
        (set `self.IsWatered` false)
        (bind _returnvalue (`SeedItem.GetStage` (`self.SeedItem`) (`self.Stage`)))
        (`StaticMeshComponent.SetStaticMesh` _crop _returnvalue)
        (add `PrimitiveComponent.OnClicked` _crop (delegate `OnClicked_Event_0`))))
    (else
      (set `self.IsWatered` false)
      (`StaticMeshComponent.SetStaticMesh` _staticmesh "/Game/MyAssets/blocks/soil.soil"))))

(event `OnClicked_Event_0`
  (params (TouchedComponent :type "PrimitiveComponent Object Reference") (ButtonPressed :type "Key Structure" :default "None"))
  (if (>= (`self.Stage`) (`SeedItem.GrowingDays` (`self.SeedItem`)))
    (`ActorComponent.K2_DestroyComponent` (`self.Crop`))
    (bind _asbp_cubical_ranch_character (cast `/Game/BP_CubicalRanchCharacter` (`GameplayStatics.GetPlayerCharacter` 0)))
    (`/Game/BP_CubicalRanchCharacter.ProgressAchievement` _asbp_cubical_ranch_character "HARVEST" 1)
    (`/Game/BP_CubicalRanchCharacter.SpendEnergy` _asbp_cubical_ranch_character 5)
    (`CubicalRanchCharacter.GiveItem` _asbp_cubical_ranch_character (`SeedItem.Product` (`self.SeedItem`)) 1)
    (set `self.SeedItem` null)
    (set `self.Stage` 0)))

(fn `PlantSeed`
  (params (SeedItem :type "SeedItem Object Reference"))
  (returns (Succes :type Boolean))
  (if (`KismetSystemLibrary.IsValid` (`self.SeedItem`))
    (return false)
    (else
      (bind _output_get (set `self.SeedItem` SeedItem))
      (bind _returnvalue (`SeedItem.GetStage` _output_get (`self.Stage`)))
      (bind _returnvalue_2 (`AddComponent|NODE_AddStaticMeshComponent-2` :`RelativeTransform` (`KismetMathLibrary.MakeTransform` (`self.TransformLocation`) (struct :`Roll` 90.0))))
      (bind _output_get_2 (set `self.Crop` _returnvalue_2))
      (`StaticMeshComponent.SetStaticMesh` _output_get_2 _returnvalue)
      (bind _asbp_cubical_ranch_character (cast `/Game/BP_CubicalRanchCharacter` (`GameplayStatics.GetPlayerCharacter` 0)))
      (`/Game/BP_CubicalRanchCharacter.ProgressAchievement` _asbp_cubical_ranch_character "PLANT" 1)
      (return true))))

(fn `UserConstructionScript`
  (`parent.UserConstructionScript`))